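; Player stats component on the ship controller, tracking health, Curse, experience and level, and gating the Dive, Eclipse and Cursed Bomb abilities.
; A LevelProgression table sets health and Curse caps, XP thresholds and the rate of timer-driven regeneration.
; Abilities check Curse plus dive state or timed cooldowns, then call the controlled Adventure or Fight ship; Cursed Bomb never deducts its cost.
; Dispatchers broadcast stat and ability changes.
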(event `ActivateComponent`
  (`self.LevelUp`)
  (bind _output_get (set `self.CurrentHP` (`.HealthPoints_2_CED8BF5D496D5D45BD9A75B8E650A0F5` (break `/Game/Developers/roman/Collections/Core/S_LevelParams` (`|GetArrayItem` (`self.LevelProgression`) (`self.CurrentLevel`))))))
  (`self.OnHealthUpdated` _output_get)
  (bind _output_get_2 (set `self.CurrentCurse` 50))
  (`self.OnCurseUpdated` _output_get_2)
  (`self.StartRegenHP`))

(event `UseDive`
  (bind _asbp_ship_adventure (cast `/Game/Developers/roman/Collections/FightShip/BP_Ship_Adventure` (`Controller.K2_GetPawn` (cast `/Game/Developers/roman/Collections/FightShip/BP_ShipController` (`self.GetOwner`) :!pure true))))
  (if (`self.IsCanUseDive` _asbp_ship_adventure)
    (bind _output_get (set `self.CurrentCurse` (- (`self.CurrentCurse`) (`self.DiveCost`))))
    (`KismetSystemLibrary.PrintString` (`KismetStringLibrary.Concat_StrStr` "Curse updated. New value: " (`KismetStringLibrary.Conv_IntToString` _output_get)))
    (`self.OnCurseUpdated` _output_get)
    (`/Game/Developers/roman/Collections/FightShip/BP_Ship_Adventure.PerformDive` _asbp_ship_adventure)))

(event `UseEclipse`
  (bind _asbp_ship_fight (cast `/Game/Developers/roman/Collections/FightShip/BP_Ship_Fight` (`Controller.K2_GetPawn` (cast `/Game/Developers/roman/Collections/FightShip/BP_ShipController` (`self.GetOwner`) :!pure true))))
  (if (`self.IsCanUseEclipse`)
    (bind _output_get (set `self.CurrentCurse` (- (`self.CurrentCurse`) (`self.EclipseCost`))))
    (set `self.EclipseCoolingdown` true)
    (`self.OnCurseUpdated` _output_get)
    (`self.OnEclipseUsed`)
    (`KismetSystemLibrary.K2_SetTimerDelegate` (`|CreateDelegate` :!event `OnEclipseCooledDownEvent`) (`self.EclipseCooldown`))
    (`KismetSystemLibrary.PrintString` "Eclipse Used")
    (`/Game/Developers/roman/Collections/FightShip/BP_Ship_Fight.PerformEclipse` _asbp_ship_fight)))

(event `OnDiveCooledDownEvent`
  (set `self.DiveCollingdown` false)
  (`self.OnDiveCooledDown`))

(event `OnEclipseCooledDownEvent`
  (set `self.EclipseCoolingdown` false)
  (`self.OnEclipseCooledDown`))

(event `UseCursedBomb`
  (bind _asbp_ship_fight (cast `/Game/Developers/roman/Collections/FightShip/BP_Ship_Fight` (`Controller.K2_GetPawn` (cast `/Game/Developers/roman/Collections/FightShip/BP_ShipController` (`self.GetOwner`) :!pure true))))
  (if (`self.IsCanUseCursedBomb`)
    (set `self.CursedBombIsCooldown` true)
    (`self.OnCurseBombUsed`)
    (`KismetSystemLibrary.K2_SetTimerDelegate` (delegate `OnCursedBombCooldownedEvent`) (`self.CursedBombCooldown`))
    (`/Game/Developers/roman/Collections/FightShip/BP_Ship_Fight.PerformCursedBomb` _asbp_ship_fight)))

(event `OnCursedBombCooldownedEvent`
  (set `self.CursedBombIsCooldown` false)
  (`self.OnCurseBombCooledDown`))

(fn `AddCurse`
  (params (Delta :type Integer))
  (bind _output_get (set `self.CurrentCurse` (`KismetMathLibrary.Clamp` (+ Delta (`self.CurrentCurse`)) 0 (`.CurseCapacity_11_4D8278CD43636953BB602F9B9AE1895B` (break `/Game/Developers/roman/Collections/Core/S_LevelParams` (`|GetArrayItem` (`self.LevelProgression`) (`self.CurrentLevel`)))))))
  (`self.OnCurseUpdated` _output_get))

(fn `AddExp`
  (params (Exp :type Integer))
  (`self.UpdateExp` (+ (`self.CurrentExp`) Exp))
  (if (>= (`self.CurrentExp`) (`.ExpToLevelUp_13_826FF6C74510CDB67B7F13843F302E25` (break `/Game/Developers/roman/Collections/Core/S_LevelParams` (`|GetArrayItem` (`self.LevelProgression`) (`self.CurrentLevel`)))))
    (`self.LevelUp`)))

(fn `IsCanUseCursedBomb`
  (returns (ReturnValue :type Boolean))
  (return (and (>= (`self.CurrentCurse`) (`self.CursedBombCost`)) (not (`self.CursedBombIsCooldown`)))))

(fn `IsCanUseDive`
  (params (Ship :type "/Game/Developers/roman/Collections/FightShip/BP_Ship_Adventure Object Reference"))
  (returns (ReturnValue :type Boolean))
  (return (and (>= (`self.CurrentCurse`) (`self.DiveCost`)) (not (`/Game/Developers/roman/Collections/FightShip/BP_Ship_Adventure.IsInDive` Ship)))))

(fn `IsCanUseEclipse`
  (returns (ReturnValue :type Boolean))
  (return (and (>= (`self.CurrentCurse`) (`self.EclipseCost`)) (not (`self.EclipseCoolingdown`)))))

(fn `LevelUp`
  (bind _output (`|GetArrayItem` (`self.LevelProgression`) (`self.CurrentLevel`)))
  (`/Engine/EditorBlueprintResources/StandardMacros.IncrementInt` (`self.CurrentLevel`)
    (:`  `
      (if (`KismetArrayLibrary.Array_IsValidIndex` (`self.LevelProgression`) (`self.CurrentLevel`))
        (`self.UpdateExp` 0)
        (`self.OnLevelUpdated` _output)
        (`GameplayStatics.SpawnSound2D` "/Game/Assets/Sounds/LevelUp.LevelUp" 1.0 1.0 0.0 null)
        (set `self.HealthRegenRate` (`.AutoRegeneration_8_60A64BD247C14727CE125698E53BFDC3` (break `/Game/Developers/roman/Collections/Core/S_LevelParams` _output)))))))

(fn `RestoreHP`
  (`self.UpdateHP` (`self.HealthRegenRate`)))

(fn `StartRegenHP`
  (bind _returnvalue (`KismetSystemLibrary.K2_SetTimerDelegate` (`|CreateDelegate` :!event `RestoreHP`) 1.0 true))
  (set `self.RestoreHPTimer` _returnvalue))

(fn `StopRegenHP`
  (`KismetSystemLibrary.K2_ClearAndInvalidateTimerHandle` (`self.RestoreHPTimer`)))

(fn `UpdateExp`
  (params (NewExp :type Integer))
  (bind _output_get (set `self.CurrentExp` NewExp))
  (`self.OnExpUpdated` _output_get))

(fn `UpdateHP`
  (params (HPDelta :type Integer))
  (bind _output_get (set `self.CurrentHP` (`KismetMathLibrary.Clamp` (+ HPDelta (`self.CurrentHP`)) -10000 (`.HealthPoints_2_CED8BF5D496D5D45BD9A75B8E650A0F5` (break `/Game/Developers/roman/Collections/Core/S_LevelParams` (`|GetArrayItem` (`self.LevelProgression`) (`self.CurrentLevel`)))))))
  (`self.OnHealthUpdated` _output_get))