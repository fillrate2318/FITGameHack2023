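; Shark actor that swims a repeating path along a spline.
; Each tick it advances a distance by Speed and delta time, then sets the Shark component's relative location and rotation from the spline's local-space transform at that distance, preserving its scale.
; The distance resets to zero once it passes the spline's length, restarting the loop.
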(event `self.ReceiveTick`
  (params (DeltaSeconds :type "Float (single-precision)"))
  (bind (_returnvalue_location _returnvalue_rotation) (`KismetMathLibrary.BreakTransform` (`SplineComponent.GetTransformAtDistanceAlongSpline` (`self.Spline`) (`self.Distance`) "Local" false)))
  (set `self.Distance` (+ (* DeltaSeconds (`self.Speed`)) (`self.Distance`)))
  (`SceneComponent.K2_SetRelativeTransform` (`self.shark`) (`KismetMathLibrary.MakeTransform` _returnvalue_location _returnvalue_rotation (`SceneComponent.RelativeScale3D` (`self.shark`))) false false)
  (if true
    (if (> (`self.Distance`) (`SplineComponent.GetSplineLength` (`self.Spline`)))
      (set `self.Distance` 0.0))))

(fn `UserConstructionScript`)